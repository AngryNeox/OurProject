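; DoorTrigger is a one-shot trigger that moves the door of a referenced SimpleDoor when a Character1 overlaps it.
; On first valid overlap it sets a Disable flag, records the Door component's relative location and plays the TimeToMove timeline.
; Each timeline update adds the track value to that start location, sliding the door without sweeping.
; An unconnected SetActorLocation node is left in the graph.
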(event `self.ReceiveActorBeginOverlap`
  (params (OtherActor :type "Actor Object Reference"))
  (bind _door (`/Game/Blueprints/SimpleDoor.Door` (`self.SimpleDoor`)))
  (if (not (`self.Disable`))
    (cast `/Game/TwinStickBP/Blueprints/Character1` OtherActor)
    (set `self.Disable` true)
    (set `self.StartLocation` (.location (`SceneComponent.GetRelativeTransform` _door)))
    (bind (_direction _newtrack_1) (`Timeline|TimeToMove`)
      (:`Update`
        (`SceneComponent.K2_SetRelativeLocation` _door (+ (`self.StartLocation`) _newtrack_1) false false)))))

(fn `UserConstructionScript`)