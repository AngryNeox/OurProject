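; RobotTest is a test pawn, apparently a robot, with side-to-side movement along the Y axis and a physics-driven jump.
; MoveRight feeds movement input, while Jump sets IsJumping and applies a large upward force to Box if a ground trace hits.
; The ground check is a short horizontal line trace along Y just below Box's center.
; Tick repeats that trace and clears IsJumping once it stops hitting, so on leaving the ground rather than landing.
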(event `InputAxis|MoveRight`
  (params (AxisValue :type "Float (single-precision)"))
  (`self.AddMovementInput` (0.0 -1.0 0.0) AxisValue))

(event `InputAction|Jump` :overrideparent false
  (params (Key :type "Key Structure"))
  (bind _returnvalue (`SceneComponent.K2_GetComponentLocation` (`self.Box`)))
  (:`Pressed`
    (if (not (`self.IsJumping`))
      (set `self.IsJumping` true)
      (bind (_outhit _returnvalue_2) (`KismetSystemLibrary.LineTraceSingle` (+ _returnvalue (0.0 -50.0 -51.0)) (+ _returnvalue (0.0 50.0 -51.0)) "TraceTypeQuery1"))
      (if _returnvalue_2
        (`PrimitiveComponent.AddForce` (`self.Box`) (0.0 0.0 10000000.0) "None" false)))))

(event `self.ReceiveTick`
  (params (DeltaSeconds :type "Float (single-precision)"))
  (bind _returnvalue (`SceneComponent.K2_GetComponentLocation` (`self.Box`)))
  (if (`self.IsJumping`)
    (bind (_outhit _returnvalue_2) (`KismetSystemLibrary.LineTraceSingle` (+ _returnvalue (0.0 -50.0 -51.0)) (+ _returnvalue (0.0 50.0 -51.0)) "TraceTypeQuery1"))
    (if (not _returnvalue_2)
      (set `self.IsJumping` false))))

(fn `UserConstructionScript`)